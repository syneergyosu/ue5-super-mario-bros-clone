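; BP_KillVolume is a box-shaped kill volume that takes a life from the player on contact in a Super Mario style game.
; On box overlap, it checks that the other actor implements BPI_Player, fetches the player reference through that interface, and calls UpdateLives with one fewer life.
; The construction script sizes the box from X, Y and Z variables.
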(event OnComponentBeginOverlap(Box)
  (params (OverlappedComponent :type Primitive%20Component%20Object%20Reference) (OtherActor :type Actor%20Object%20Reference) (OtherComp :type Primitive%20Component%20Object%20Reference) (OtherBodyIndex :type Integer) (bFromSweep :type Boolean) (SweepResult :type Hit%20Result%20Structure%20%28by%20ref%29))
  ;[0.05098 0.05098 0.05098] If player hits box collision remove live
  (if (Utilities|DoesObjectImplementInterface OtherActor "/Game/_SuperMario/Blueprints/Interfaces/BPI_Player.BPI_Player_C")
    (bind _reference (Class|BPIPlayer|GetPlayerReference(Message) OtherActor))
    (Default|UpdateLives _reference (- (Variables|/Game/ThirdPerson/Blueprints/BP_ThirdPersonCharacter.BP_ThirdPersonCharacter_C|GetLives _reference) 1))))

(fn ConstructionScript
  (Components|Box|SetBoxExtent (Variables|Default|GetBox) (Math|Vector|MakeVector (Variables|Shape|GetX) (Variables|Shape|GetY) (Variables|Shape|GetZ)) true))