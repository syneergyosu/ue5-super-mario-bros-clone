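; BP_Block is a Mario-style block that bumps up and down when a player hits it.
; A mesh hit from an actor implementing BPI_Player plays the bump sound, raises the mesh, then lowers it after a short delay.
; Two timelines drive the motion, lerping from the mesh's current world location on each update, so offsets accumulate rather than following fixed endpoints.
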(event OnComponentHit(StaticMesh)
  (params (HitComponent :type Primitive%20Component%20Object%20Reference) (OtherActor :type Actor%20Object%20Reference) (OtherComp :type Primitive%20Component%20Object%20Reference) (NormalImpulse :type Vector :default "0, 0, 0") (Hit :type Hit%20Result%20Structure%20%28by%20ref%29))
  (if (Utilities|DoesObjectImplementInterface OtherActor "/Game/_SuperMario/Blueprints/Interfaces/BPI_Player.BPI_Player_C")
    (Audio|PlaySound2D "/Game/_SuperMario/Assets/Audio/smb_bump.smb_bump" 1.0 1.0 0.0 0 0)
    (CallFunction|MoveUp)
    (Utilities|FlowControl|Delay 0.15)
    (CallFunction|MoveDown)))

(event Custom|MoveUp
  (bind _staticmesh (Variables|Default|GetStaticMesh))
  (bind _returnvalue (Transformation|GetWorldLocation _staticmesh))
  ;[0.05098 0.05098 0.05098] Block Goes Up And Down
  (bind _alpha (Timeline|T_Up PlayFromStart)
    (:Update
      (Transformation|SetWorldLocation _staticmesh (Math|Vector|Lerp(Vector) _returnvalue (+ _returnvalue "0.000000,0.000000,5.000000") _alpha) false false))))

(event Custom|MoveDown
  (bind _staticmesh (Variables|Default|GetStaticMesh))
  (bind _returnvalue (Transformation|GetWorldLocation _staticmesh))
  ;[0.05098 0.05098 0.05098] Block Goes Up And Down
  (bind _alpha (Timeline|Timeline PlayFromStart)
    (:Update
      (Transformation|SetWorldLocation _staticmesh (Math|Vector|Lerp(Vector) _returnvalue (- _returnvalue "0.000000,0.000000,5.000000") _alpha) false false))))

(fn ConstructionScript)